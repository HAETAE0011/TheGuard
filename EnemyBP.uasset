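; Enemy Blueprint with clamped health, a toggleable target-lock visual and an execution state at low health.
; TakeDamage updates Health and a percentage, and BeginPlay hands the enemy reference to its health widget.
; Tick polls Health and, once at the low threshold, flags the enemy killable and calls LowEnemyHealth.
; SendTargetLocation copies TargetLocation into the Zone game instance, and Killed plays a death animation.
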(event EventBeginPlay
  (bind _asenemy_health (Utilities|Casting|CastToenemyHealth (UserInterface|GetUserWidgetObject (Variables|Default|GetEnemyHealthUI))))
  (Variables|/Game/enemyHealth.enemyHealth_C|SetEnemy _asenemy_health self))

(event EventTargetLockON
  (bind _targetvisual (Variables|Default|GetTargetVisual))
  (Utilities|FlowControl|FlipFlop
    (:A
      (Development|SetHiddeninGame _targetvisual false false))
    (:B
      (Development|SetHiddeninGame _targetvisual true false))))

(event EventTick
  (params (DeltaSeconds :type Float%20%28single-precision%29))
  (if (<= (Variables|Default|GetHealth) 2e+01)
    (Utilities|FlowControl|DoOnce false
      (:Completed
        (Variables|Default|SetcanBeKilled? true)
        (CallFunction|LowEnemyHealth)
        (Development|PrintString "executable!")))))

(fn ConstructionScript)

(fn TakeDamage
  (params (damage :type Float%20%28single-precision%29))
  (bind _output_get (Variables|Default|SetHealth (Math|Float|Clamp(Float) (- (Variables|Default|GetHealth) damage) 0.0 1e+02)))
  (Variables|Default|SetHealthPercentage (/ _output_get 1e+02)))

(fn SendTargetLocation
  (bind _aszone_gi (Utilities|Casting|CastToZone_GI (Game|GetGameInstance)))
  (bind _output_get (Variables|/Game/ThirdPersonBP/Blueprints/Zone_GI.Zone_GI_C|SetTargetPosition _aszone_gi (Variables|Default|Gettarget%20location)))
  (Variables|Default|Settarget%20location _output_get))

(fn Killed
  (Development|PrintString "Hello")
  (Components|Animation|PlayAnimation (Variables|Character|GetMesh) "/Game/Death_3.Death_3" false))